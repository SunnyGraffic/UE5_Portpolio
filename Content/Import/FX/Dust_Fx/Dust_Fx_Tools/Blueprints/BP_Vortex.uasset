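; BP_Vortex is a placeable dust FX actor that configures a spline-driven vortex effect.
; Its construction script passes the actor's Spline component to the VortexEnv effect as an object variable, so the effect can read the path.
; It also pushes exposed color, look, size, spawn rate, velocity and slow-motion settings into the effect's parameters.
; The event graph is empty, with no runtime logic.
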(fn `UserConstructionScript`
  (bind _vortexenv (`self.VortexEnv`))
  (bind _vortexenv_2 (`self.VortexEnv`))
  (bind _vortexenv_3 (`self.VortexEnv`))
  (bind _vortexenv_4 (`self.VortexEnv`))
  (bind _vortexenv_5 (`self.VortexEnv`))
  (`NiagaraComponent.SetVariableObject` (`self.VortexEnv`) "spline" (`self.Spline`))
  (`NiagaraComponent.SetVariableLinearColor` _vortexenv_3 "Color_A" (`self.Color_A`))
  (`NiagaraComponent.SetVariableLinearColor` _vortexenv_3 "Color_B" (`self.Color_B`))
  (`NiagaraComponent.SetVariableFloat` _vortexenv_4 "Constrast" (`self.Constrast`))
  (`NiagaraComponent.SetVariableFloat` _vortexenv_4 "Emessive" (`self.Emessive`))
  (`NiagaraComponent.SetVariableFloat` _vortexenv_5 "SlowMotion" (`self.SlowMotion`))
  (`NiagaraComponent.SetVariableFloat` _vortexenv_5 "Normal" (`self.Normal`))
  (`NiagaraComponent.SetVariableFloat` _vortexenv "Opacity" (`self.Opacity`))
  (`NiagaraComponent.SetVariableFloat` _vortexenv "Size" (`self.Size`))
  (`NiagaraComponent.SetVariableFloat` _vortexenv_2 "SpawnRate" (`self.SpawnRate`))
  (`NiagaraComponent.SetVariableFloat` _vortexenv_2 "velocity" (`self.velocity`)))