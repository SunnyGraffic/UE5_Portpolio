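; Spline-based gas or smoke effect actor driven by a Niagara component named Smoke.
; The construction script passes the spline and the exposed look and emission settings, such as colors, size, spawn rate, lifetime and velocity, into the effect's user variables.
; When FastSimulation is set, BeginPlay runs a timeline whose track value sets how far the simulation advances on each update, speeding up the smoke.
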(event `self.ReceiveBeginPlay`
  (if (`self.FastSimulation`)
    (bind (_direction _newtrack_0) (`Timeline|Timeline_0`)
      (:`Update`
        (`NiagaraComponent.AdvanceSimulationByTime` (`self.Smoke`) _newtrack_0 (`GameplayStatics.GetWorldDeltaSeconds`))))))

(fn `UserConstructionScript`
  (bind _smoke (`self.Smoke`))
  (bind _smoke_2 (`self.Smoke`))
  (bind _smoke_3 (`self.Smoke`))
  (bind _smoke_4 (`self.Smoke`))
  (bind _smoke_5 (`self.Smoke`))
  (`NiagaraComponent.SetVariableObject` _smoke "sp" (`self.Spline`))
  (`NiagaraComponent.SetVariableLinearColor` _smoke "Color_A" (`self.Color_A`))
  (`NiagaraComponent.SetVariableLinearColor` _smoke "Color_B" (`self.Color_B`))
  (`NiagaraComponent.SetVariableFloat` _smoke_4 "Constrast" (`self.Constrast`))
  (`NiagaraComponent.SetVariableFloat` _smoke_4 "Emessive" (`self.Emessive`))
  (`NiagaraComponent.SetVariableFloat` _smoke_2 "LifeTime" (`self.LifeTime`))
  (`NiagaraComponent.SetVariableFloat` _smoke_2 "Normal" (`self.Normal`))
  (`NiagaraComponent.SetVariableFloat` _smoke_5 "Opacity" (`self.Opacity`))
  (`NiagaraComponent.SetVariableFloat` _smoke_5 "Size" (`self.Size`))
  (`NiagaraComponent.SetVariableFloat` _smoke_3 "SpawnRate" (`self.SpawnRate`))
  (`NiagaraComponent.SetVariableFloat` _smoke_3 "velocity" (`self.velocity`)))