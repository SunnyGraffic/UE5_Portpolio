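; BP_ProjectileTest is a test projectile for FX that bursts when its sphere overlaps an actor tagged COLLISION.
; The skeletal mesh and decal start hidden; on impact both are revealed and projectile movement stops.
; Timelines then dissolve the projectile effect, animate the decal's dissolve through a dynamic material and scrub the mesh's animation position.
; It also spawns the NS_BombTest Niagara system at the sphere and destroys itself after a short delay.
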(event `self.ReceiveBeginPlay`
  (bind _returnvalue (`DecalComponent.CreateDynamicMaterialInstance` (`self.Decal`)))
  (`MaterialInstanceDynamic.SetScalarParameterValue` _returnvalue "Dissolve" 1.0)
  (`SceneComponent.SetHiddenInGame` (`self.SKM`) true false)
  (`SceneComponent.SetHiddenInGame` (`self.Decal`) true false))

(event `self.Sphere.OnComponentBeginOverlap`
  (params (OverlappedComponent :type "PrimitiveComponent Object Reference") (OtherActor :type "Actor Object Reference") (OtherComp :type "PrimitiveComponent Object Reference") (OtherBodyIndex :type Integer) (bFromSweep :type Boolean) (SweepResult :type "HitResult Structure (by ref)"))
  (bind _skm (`self.SKM`))
  (if (`self.ActorHasTag` OtherActor "COLLISION")
    (`SceneComponent.SetHiddenInGame` (`self.SKM`) false false)
    (`SceneComponent.SetHiddenInGame` (`self.Decal`) false false)
    (`MovementComponent.StopMovementImmediately` (`self.ProjectileMovement`))
    (`|ExecutionSequence`
      (:`then_0`
        (bind (_direction _dissolve) (`Timeline|Dissolve_Projectile` :!via `PlayFromStart`)
          (:`Update`
            (`FXSystemComponent.SetFloatParameter` (`self.Projectile`) "Dissolve" _dissolve))))
      (:`then_1`
        (`NiagaraFunctionLibrary.SpawnSystemAtLocation` "/Game/FX/Test_Projectile/NS_BombTest.NS_BombTest" (`SceneComponent.K2_GetComponentLocation` (`self.Sphere`))))
      (:`then_2`
        (`KismetSystemLibrary.Delay` 0.0)
        (bind (_direction_2 _dissolve_2) (`Timeline|Decal_Spawn` :!via `PlayFromStart`)
          (:`Update`
            (`MaterialInstanceDynamic.SetScalarParameterValue` (stale `self.ReceiveBeginPlay` _returnvalue) "Dissolve" _dissolve_2))))
      (:`then_3`
        (`KismetSystemLibrary.Delay` 0.0)
        (bind (_direction_3 _animation) (`Timeline|타임라인` :!via `PlayFromStart`)
          (:`Update`
            (`SkeletalMeshComponent.SetPosition` _skm _animation true)
            (`MeshComponent.SetScalarParameterValueOnMaterials` _skm "Dissolve" 0.0))))
      (:`then_4`
        (`KismetSystemLibrary.Delay` 2.0)
        (`self.K2_DestroyActor`)))))

(fn `UserConstructionScript`)